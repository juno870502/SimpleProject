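; BP_ArrowRain is an arrow rain attack actor that shows a magic circle, then emits arrow particles at its location.
; A delayed sequence, started on BeginPlay or by CustomEvent, spawns the emitters, then a timeline drives the circle's opacity through a dynamic material before cleanup and self-destruction.
; Arrow particle collisions drive the hits, spawning smoke at each impact and applying radial damage only on the authority.
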(event Custom|CustomEvent
  (params (Location :type Vector))
  (bind _returnvalue (Transformation|GetActorLocation))
  (Effects|SpawnEmitteratLocation "/Game/HuntingGround/Arrow/P_MagicCicle_Spon.P_MagicCicle_Spon" _returnvalue)
  (Utilities|FlowControl|Delay 0.5)
  (bind _returnvalue_2 (Effects|SpawnEmitteratLocation "/Game/HuntingGround/Arrow/P_MagicCicle.P_MagicCicle" _returnvalue))
  (Utilities|Array|Add (Variables|Default|GetParticle) _returnvalue_2)
  (Utilities|FlowControl|Delay 2.0)
  (bind _returnvalue_3 (Effects|SpawnEmitteratLocation "/Game/HuntingGround/Arrow/P_Arrow.P_Arrow" _returnvalue))
  (Utilities|Array|Add (Variables|Default|GetParticle) _returnvalue_3)
  (EventDispatchers|BindEventtoOnParticleCollide _returnvalue_3 (delegate Custom|OnParticleCollide))
  (Utilities|FlowControl|Delay 2.0)
  (bind _returnvalue_4 (Rendering|Material|CreateDynamicMaterialInstance _returnvalue_2 0 "/Game/HuntingGround/Arrow/M_Magie_Inst.M_Magie_Inst" "None" :!class /Script/Engine.PrimitiveComponent))
  (bind _opacity (Timeline|타임라인_1 Play)
    (:Update
      (Rendering|Material|SetScalarParameterValue _returnvalue_4 "Opasity_Alpha_Max" _opacity :!class /Script/Engine.MaterialInstanceDynamic))
    (:Finished
      (for _array_element (Variables|Default|GetParticle)
        (Components|DestroyComponent _array_element)
        (Actor|DestroyActor)))))

(event Custom|OnParticleCollide
  (params (EventName :type Name) (EmitterTime :type Float%20%28single-precision%29) (ParticleTime :type Integer) (Location :type Vector) (Velocity :type Vector) (Direction :type Vector) (Normal :type Vector) (BoneName :type Name) (PhysMat :type Physical%20Material%20Object%20Reference))
  (Effects|SpawnEmitteratLocation "/Game/HuntingGround/Arrow/P_Smoke.P_Smoke" Location)
  (Networking|SwitchHasAuthority
    (:Authority
      (Game|Damage|ApplyRadialDamage 1e+01 Location 1e+02 "/Script/SimpleProject.BasicArrowRainDamageType" 0 0 0 false "ECC_Visibility"))))

(event EventBeginPlay
  (bind _returnvalue (Transformation|GetActorLocation))
  (Effects|SpawnEmitteratLocation "/Game/HuntingGround/Arrow/P_MagicCicle_Spon.P_MagicCicle_Spon" _returnvalue)
  (Utilities|FlowControl|Delay 0.5)
  (bind _returnvalue_2 (Effects|SpawnEmitteratLocation "/Game/HuntingGround/Arrow/P_MagicCicle.P_MagicCicle" _returnvalue))
  (Utilities|Array|Add (Variables|Default|GetParticle) _returnvalue_2)
  (Utilities|FlowControl|Delay 2.0)
  (bind _returnvalue_3 (Effects|SpawnEmitteratLocation "/Game/HuntingGround/Arrow/P_Arrow.P_Arrow" _returnvalue))
  (Utilities|Array|Add (Variables|Default|GetParticle) _returnvalue_3)
  (EventDispatchers|BindEventtoOnParticleCollide _returnvalue_3 (delegate Custom|OnParticleCollide))
  (Utilities|FlowControl|Delay 2.0)
  (bind _returnvalue_4 (Rendering|Material|CreateDynamicMaterialInstance _returnvalue_2 0 "/Game/HuntingGround/Arrow/M_Magie_Inst.M_Magie_Inst" "None" :!class /Script/Engine.PrimitiveComponent))
  (bind _opacity (Timeline|타임라인_1 Play)
    (:Update
      (Rendering|Material|SetScalarParameterValue _returnvalue_4 "Opasity_Alpha_Max" _opacity :!class /Script/Engine.MaterialInstanceDynamic))
    (:Finished
      (for _array_element (Variables|Default|GetParticle)
        (Components|DestroyComponent _array_element)
        (Actor|DestroyActor)))))

(fn ConstructionScript)